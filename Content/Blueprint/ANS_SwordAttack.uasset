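; Anim notify state that runs hit detection for a sword attack while its animation window is active.
; Each tick it sphere-traces on Visibility between two right-hand sockets, with debug drawing left on.
; A blocking hit on a BPI_Attack actor sends AttackMessage, then calls JumpReset on player 0's BP_ThirdPersonCharacter.
; Notify begin calls OnceReset on that same character, regardless of which mesh plays the animation.
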(fn `Received_NotifyBegin`
  (params (MeshComp :type "SkeletalMeshComponent Object Reference") (Animation :type "AnimSequenceBase Object Reference") (TotalDuration :type "Float (single-precision)") (EventReference :type "AnimNotifyEventReference Structure (by ref)"))
  (returns (ReturnValue :type Boolean))
  (bind _asbp_third_person_character (cast `/Game/ThirdPerson/Blueprints/BP_ThirdPersonCharacter` (`GameplayStatics.GetPlayerCharacter` MeshComp)))
  (`/Game/ThirdPerson/Blueprints/BP_ThirdPersonCharacter.OnceReset` _asbp_third_person_character)
  (return false))

(fn `Received_NotifyTick`
  (params (MeshComp :type "SkeletalMeshComponent Object Reference") (Animation :type "AnimSequenceBase Object Reference") (FrameDeltaTime :type "Float (single-precision)") (EventReference :type "AnimNotifyEventReference Structure (by ref)"))
  (returns (ReturnValue :type Boolean))
  (bind _outhit (`KismetSystemLibrary.SphereTraceSingle` :`WorldContextObject` MeshComp :`Start` (`SceneComponent.GetSocketLocation` MeshComp "hand_rSocket") :`End` (`SceneComponent.GetSocketLocation` MeshComp "hand_rSocket_0") :`Radius` 25.0 :`TraceChannel` "TraceTypeQuery1" :`DrawDebugType` "ForDuration" :`DrawTime` 2.0))
  (if (and (`GameplayStatics.BreakHitResult` _outhit) (`KismetSystemLibrary.DoesImplementInterface` (`.HitActor` (`GameplayStatics.BreakHitResult` _outhit)) "/Game/ThirdPerson/Blueprints/BPI_Attack.BPI_Attack_C"))
    (message `/Game/ThirdPerson/Blueprints/BPI_Attack.Attack` (`.HitActor` (`GameplayStatics.BreakHitResult` _outhit)))
    (bind _asbp_third_person_character (cast `/Game/ThirdPerson/Blueprints/BP_ThirdPersonCharacter` (`GameplayStatics.GetPlayerCharacter` MeshComp)))
    (`/Game/ThirdPerson/Blueprints/BP_ThirdPersonCharacter.Jump reset` _asbp_third_person_character)
    (return false)))